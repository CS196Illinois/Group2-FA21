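; Pivot sphere actor that the player spins in either direction around one axis by holding Z or C.
; Each key sets a signed Rate and plays the shared Rotate timeline, whose alpha linearly scales the RotatingMovement rotation rate.
; Key release zeroes the rotation rate without stopping the timeline, and the Reverse branches are unreachable behind constant-true conditions.
; Input from player controller 0 is re-enabled every Tick.
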(event EventTick
  (params (DeltaSeconds :type Float%20%28single-precision%29))
  (Input|EnableInput (Game|GetPlayerController 0)))

(event Collision|EventActorBeginOverlap
  (params (OtherActor :type Actor%20Object%20Reference)))

(event Input|KeyboardEvents|Z
  (params (Key :type Key%20Structure :default "None"))
  (:Pressed
    (if true
      (Variables|Default|SetRate 1e+01)
      (bind _alpha (Timeline|Rotate PlayFromStart)
        (:Update
          (Variables|/Script/Engine.RotatingMovementComponent|SetRotationRate (Variables|Default|GetRotatingMovement) (Math|Rotator|MakeRotator 0.0 (Math|Interpolation|Ease "Linear" _alpha 0.0 (Variables|Default|GetRate)) 0.0))))
      (else
        (Timeline|Rotate Reverse))))
  (:Released
    (Variables|/Script/Engine.RotatingMovementComponent|SetRotationRate (Variables|Default|GetRotatingMovement) "0, 0, 0")))

(event Input|KeyboardEvents|C
  (params (Key :type Key%20Structure :default "None"))
  (:Pressed
    (if true
      (Variables|Default|SetRate -1e+01)
      (bind _alpha (Timeline|Rotate PlayFromStart)
        (:Update
          (Variables|/Script/Engine.RotatingMovementComponent|SetRotationRate (Variables|Default|GetRotatingMovement) (Math|Rotator|MakeRotator 0.0 (Math|Interpolation|Ease "Linear" _alpha 0.0 (Variables|Default|GetRate)) 0.0))))
      (else
        (Timeline|Rotate Reverse))))
  (:Released
    (Variables|/Script/Engine.RotatingMovementComponent|SetRotationRate (Variables|Default|GetRotatingMovement) "0, 0, 0")))

(fn ConstructionScript)